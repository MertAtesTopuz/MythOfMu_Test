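; Player controller for a top-down building game with a camera pawn, cursor-driven building placement and a main UI widget.
; It forwards input to the pawn's movement component for movement, edge scroll, zoom, gated panning and resets.
; Each tick a cursor trace, scaled with camera arm length, feeds the building manager, which also receives preview selection and rotation.
; It relays date-time and game-speed events to the UI and game state.
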(event `Key|B`
  (params (Key :type "Key Structure"))
  (:`Pressed`
    (`/Game/Core/Buildings/BP_BuildingManager.SetPreview` (`self.BP_BuildingManager`) "Barracks")))

(event `self.ReceiveBeginPlay`
  (`|ExecutionSequence`
    (:`then_0`
      (set `self.bShowMouseCursor` true)
      (bind _asbp_camera_pawn (cast `/Game/Core/Player/BP_CameraPawn` (`GameplayStatics.GetPlayerPawn` 0)))
      (bind _output_get (set `self.CameraPawnRef` _asbp_camera_pawn))
      (set `self.CameraMovementRef` (`/Game/Core/Player/BP_CameraPawn.BP_PawnMovementComp` _output_get)))
    (:`then_1`
      (bind _returnvalue (`|CreateWidget` "/Game/Core/Widgets/WBP_MainUI.WBP_MainUI_C" self))
      (bind _output_get_2 (set `self.MainWidgetRef` _returnvalue))
      (`UserWidget.AddToViewport` _output_get_2 0)
      (`WidgetBlueprintLibrary.SetInputMode_GameAndUIEx` self _output_get_2 "LockInFullscreen" false))))

(event `self.ReceiveTick`
  (params (DeltaSeconds :type "Float (single-precision)"))
  (bind _output_get (set `self.MousePosition` (`self.SetMousePosition` (+ (`/Game/Core/Player/BP_CameraPawn.GetCurrentArmLength` (`self.CameraPawnRef`)) 2000.0))))
  (`/Game/Core/Buildings/BP_BuildingManager.SetMousePosition` (`self.BP_BuildingManager`) _output_get))

(event `InputAxisKey|MouseX` :paused true
  (params (AxisValue :type "Float (single-precision)"))
  ;[1 1 1] Edge Scroll
  (`/Game/Core/Player/BP_PawnMovementComp.EdgeScroll` (`self.CameraMovementRef`) :!label _label))

(event `InputAxis|MoveForward`
  (params (AxisValue :type "Float (single-precision)"))
  ;[1 1 1] WASD Movement
  (`/Game/Core/Player/BP_PawnMovementComp.BasicMovementControls` (`self.CameraMovementRef`) AxisValue (stale `InputAxis|MoveRight` AxisValue) :!label _label_2))

(event `InputAxisKey|MouseY` :paused true
  (params (AxisValue :type "Float (single-precision)"))
  ;[1 1 1] Edge Scroll
  (goto _label))

(event `InputAxis|MoveRight`
  (params (AxisValue :type "Float (single-precision)"))
  ;[1 1 1] WASD Movement
  (goto _label_2))

(event `InputAction|ZoomIn`
  (params (Key :type "Key Structure"))
  ;[1 1 1] Zoom Events
  (:`Pressed`
    (`/Game/Core/Player/BP_PawnMovementComp.ZoomIn` (`self.CameraMovementRef`))))

(event `InputAction|SpeedModifier`
  (params (Key :type "Key Structure"))
  (bind _cameramovementref (`self.CameraMovementRef`))
  ;[1 1 1] Speed Modifier
  (:`Pressed`
    (`/Game/Core/Player/BP_PawnMovementComp.SetSpeedModifier` _cameramovementref 2.0))
  (:`Released`
    (`/Game/Core/Player/BP_PawnMovementComp.SetSpeedModifier` _cameramovementref 1.0)))

(event `InputAction|ZoomOut`
  (params (Key :type "Key Structure"))
  ;[1 1 1] Zoom Events
  (:`Pressed`
    (`/Game/Core/Player/BP_PawnMovementComp.ZoomOut` (`self.CameraMovementRef`))))

(event `InputAction|ZoomReset`
  (params (Key :type "Key Structure"))
  ;[1 1 1] Zoom Events
  (:`Pressed`
    (`/Game/Core/Player/BP_PawnMovementComp.ResetZoom` (`self.CameraMovementRef`))))

(event `InputAxisKey|MouseX` :paused true
  (params (AxisValue :type "Float (single-precision)"))
  ;[1 1 1] Pan
  (`/Engine/EditorBlueprintResources/StandardMacros.Gate` true :!label _label_3
    (:`Exit`
      (`/Game/Core/Player/BP_PawnMovementComp.PanCamera` (`self.CameraMovementRef`) (* AxisValue (`self.PanSensitivity`))))))

(event `InputAction|Pan`
  (params (Key :type "Key Structure"))
  (bind _cameramovementref (`self.CameraMovementRef`))
  ;[1 1 1] Pan
  (:`Pressed`
    (`/Game/Core/Player/BP_PawnMovementComp.SetDisableEdgeScroll` _cameramovementref true)
    (goto _label_3 :!via `Open`))
  (:`Released`
    (`/Game/Core/Player/BP_PawnMovementComp.SetDisableEdgeScroll` _cameramovementref false)
    (goto _label_3 :!via `Close`)))

(event `InputAction|PanReset`
  (params (Key :type "Key Structure"))
  ;[1 1 1] Reset Pan
  (:`Pressed`
    (`/Game/Core/Player/BP_PawnMovementComp.ResetPan` (`self.CameraMovementRef`))))

(event `InputAction|ResetCamera`
  (params (Key :type "Key Structure"))
  ;[1 1 1] Reset Pan and Zoom
  (:`Pressed`
    (`/Game/Core/Player/BP_PawnMovementComp.ResetCamera` (`self.CameraMovementRef`))))

(event `/Game/Core/Interfaces/BPI_GameTime.SetDateTime`
  (params (DateTimeStruct :type "DateTime Structure"))
  ;[1 1 1] Set Date Time
  (message `/Game/Core/Interfaces/BPI_GameTime.SetDateTime` (`self.MainWidgetRef`) DateTimeStruct))

(event `/Game/Core/Interfaces/BPI_GameTime.UpdateGameSpeed`
  (params (NewSpeedMultiplier :type "Float (double-precision)"))
  ;[1 1 1] Update GameSpeed
  (message `/Game/Core/Interfaces/BPI_GameTime.UpdateGameSpeed` (`GameplayStatics.GetGameState`) NewSpeedMultiplier))

(event `/Game/Core/Interfaces/BPI_GameTime.SetGameSpeedInt`
  (params (GameSpeed :type "Float (double-precision)"))
  ;[1 1 1] Set Game Speed
  (message `/Game/Core/Interfaces/BPI_GameTime.SetGameSpeedInt` (`self.MainWidgetRef`) GameSpeed))

(event `InputAction|RotatePreviewLeft`
  (params (Key :type "Key Structure"))
  ;[1 1 1] Rotate Preview
  (:`Pressed`
    (`/Game/Core/Buildings/BP_BuildingManager.RotatePreviewLeft` (`self.BP_BuildingManager`))))

(event `InputAction|RotatePreviewRight`
  (params (Key :type "Key Structure"))
  ;[1 1 1] Rotate Preview
  (:`Pressed`
    (`/Game/Core/Buildings/BP_BuildingManager.RotatePreviewRight` (`self.BP_BuildingManager`))))

(fn `SetMousePosition`
  (params (TraceDistance :type "Float (double-precision)"))
  (returns (RelativeCursorLocation :type "Vector Structure"))
  (bind (_worldlocation _worlddirection) (`self.DeprojectMousePositionToWorld`))
  (bind _outhit (`KismetSystemLibrary.LineTraceSingle` _worldlocation (+ _worldlocation (* _worlddirection TraceDistance)) "TraceTypeQuery3"))
  (bind (_bblockinghit _binitialoverlap _time _distance _location _impactpoint _normal _impactnormal _physmat _hitactor) (`GameplayStatics.BreakHitResult` _outhit))
  (if (!= _hitactor null)
    (return _location)))

(fn `SetMousePosition2`
  (`|SpawnActorFromClass` "/Game/Core/Buildings/BP_BuildingMaster.BP_BuildingMaster_C" (`KismetMathLibrary.MakeTransform` (`.Location` (`GameplayStatics.BreakHitResult` (`self.GetHitResultUnderCursorByChannel` (`GameplayStatics.GetPlayerController` 0) "TraceTypeQuery1" true)))) "AlwaysSpawn" "MultiplyWithRoot" null "Null" "NewEnumerator0" null))

(fn `UserConstructionScript`)