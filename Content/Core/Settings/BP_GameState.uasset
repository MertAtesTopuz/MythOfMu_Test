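; Game state that runs the in-game clock and calendar at an adjustable game speed.
; Each Tick, unless speed is zero, it advances GameTime in hours, derives time of day and rolls days into months and years.
; It pushes GameTime to the BP_SunRotation actor found at BeginPlay, and a DateTime struct and speed to player controller 0 through messages.
; UpdateGameSpeed scales the default speed by a multiplier and calls GameSpeedControl.
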(event `self.ReceiveBeginPlay`
  (`self.SetInitialGameTime`)
  (`self.GetSunRotationActor`))

(event `GetSunRotationActor`
  (bind _outactors (`GameplayStatics.GetAllActorsOfClass` "/Game/Core/Actor/BP_SunRotation.BP_SunRotation_C"))
  (for _array_element _outactors
    (set `self.SunActorRef` _array_element)
    (break)))

(event `self.ReceiveTick`
  (params (DeltaSeconds :type "Float (single-precision)"))
  (if (!= (`self.GameSpeed`) 0.0)
    (`self.CalculateTime` DeltaSeconds)
    (`self.SetClockCalander`)
    (`self.PassGameTime`)
    (`self.PassDateTimeStruct`)
    (`self.PassGameSpeed`)))

(event `CalculateTime`
  (params (DeltaTime :type "Float (double-precision)"))
  (bind (_outgametime _daycounter) (`/Game/Core/Library/BP_GameTimeLibrary.CalculateGameTime` DeltaTime (`self.GameSpeed`) (`self.GameTime`)))
  (set `self.GameTime` _outgametime)
  (set `self.DayCounter` _daycounter))

(event `SetClockCalander`
  (bind (_year _month _day _hours _munites _seconds) (`self.UpdateClockCalander`))
  (`self.SetDateTimeStruct` _year _month _day _hours _munites _seconds))

(event `PassGameTime`
  (bind _sunactorref (`self.SunActorRef`)
    (:`then`
      (message `/Game/Core/Interfaces/BPI_GameTime.SetGameTime` _sunactorref (`self.GameTime`)))
    (:`else`)))

(event `/Game/Core/Interfaces/BPI_GameTime.UpdateGameSpeed`
  (params (NewSpeedMultiplier :type "Float (double-precision)"))
  (bind _output_get (set `self.GameSpeed` (* NewSpeedMultiplier (`self.DefultGameSpeed`))))
  (`self.GameSpeedControl` _output_get))

(event `PassDateTimeStruct`
  (message `/Game/Core/Interfaces/BPI_GameTime.SetDateTime` (`GameplayStatics.GetPlayerController` 0) (`self.DateTimeStruct`)))

(event `PassGameSpeed`
  (message `/Game/Core/Interfaces/BPI_GameTime.SetGameSpeedInt` (`GameplayStatics.GetPlayerController` 0) (`self.GameSpeed`)))

(fn `DebugingPrintGameTime`
  (params (Hour :type "Integer (by ref)") (Munite :type "Integer (by ref)") (Second :type "Integer (by ref)") (Day :type "Integer (by ref)") (Month :type "Integer (by ref)") (Year :type "Integer (by ref)"))
  (`KismetSystemLibrary.PrintString` (`KismetStringLibrary.Concat_StrStr` (`KismetStringLibrary.Conv_IntToString` Day) ":" (`KismetStringLibrary.Conv_IntToString` Month) ":" (`KismetStringLibrary.Conv_IntToString` Year) "     " (`KismetStringLibrary.Conv_IntToString` Second) "/" (`KismetStringLibrary.Conv_IntToString` Munite) "/" (`KismetStringLibrary.Conv_IntToString` Hour))))

(fn `SetDateTimeStruct`
  (params (Year :type "Integer (by ref)") (Month :type "Integer (by ref)") (Day :type "Integer (by ref)") (Hour :type "Integer (by ref)") (Minute :type "Integer (by ref)") (Second :type "Integer (by ref)"))
  (set `self.DateTimeStruct` (`KismetMathLibrary.MakeDateTime` Year Month Day Hour Minute Second)))

(fn `SetInitialGameTime`
  (set `self.GameTime` (+ (`self.Hours`) (/ (`self.Munites`) 60) (/ (`self.Seconds`) 3600.0))))

(fn `UpdateClockCalander`
  (returns (Year :type Integer) (Month :type Integer) (Day :type Integer) (Hours :type Integer) (Munites :type Integer) (Seconds :type Integer))
  (bind (_remainder _returnvalue) (`KismetMathLibrary.FMod` (* (`self.GameTime`) 3600.0) 60.0))
  (bind (_remainder_2 _returnvalue_2) (`KismetMathLibrary.FMod` (`KismetMathLibrary.Conv_IntToDouble` _returnvalue) 60.0))
  ;[1 1 1] Set Seconds
  (set `self.Seconds` (`KismetMathLibrary.FFloor` _remainder))
  ;[1 1 1] Set Munites
  (set `self.Munites` (`KismetMathLibrary.FFloor` _remainder_2))
  ;[1 1 1] Set Hours
  (set `self.Hours` (`KismetMathLibrary.FFloor` (`KismetMathLibrary.FMod` (`KismetMathLibrary.Conv_IntToDouble` _returnvalue_2) 24.0)))
  ;[1 1 1] Callander
  (bind _output_get (set `self.Day` (+ (`self.DayCounter`) (`self.Day`))))
  (if (> _output_get (`KismetMathLibrary.DaysInMonth` (`self.Year`) (`self.Month`)))
    (set `self.Day` 1)
    (set `self.Month` (+ (`self.Month`) 1)))
  (if (> (`self.Month`) 12)
    (set `self.Month` 1)
    (set `self.Year` (+ (`self.Year`) 1)))
  (return (`self.Year`) (`self.Month`) (`self.Day`) (`self.Hours`) (`self.Munites`) (`self.Seconds`)))

(fn `UserConstructionScript`)